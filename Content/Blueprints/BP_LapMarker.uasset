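; BP_LapMarker is a race lap marker that gives visual feedback when a BP_SportsCar_Pawn drives through it.
; An overlap calls HitLapMarker on the LapMarker component, which holds the lap logic outside this graph.
; A successful hit switches both checkpoint visualizers' material color parameter, then resets it after a short delay.
; The component's OnFinish event activates left and right spark effects and prints a race-finished message.
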(event `self.LapMarker.OnComponentBeginOverlap`
  (params (OverlappedComponent :type "PrimitiveComponent Object Reference") (OtherActor :type "Actor Object Reference") (OtherComp :type "PrimitiveComponent Object Reference") (OtherBodyIndex :type Integer) (bFromSweep :type Boolean) (SweepResult :type "HitResult Structure (by ref)"))
  ;[1 1 1] On Lap Marker Hit..
  (cast `/Game/VehicleTemplate/Blueprints/SportsCar/BP_SportsCar_Pawn` OtherActor)
  (bind _returnvalue (`LapMarkerComponent.HitLapMarker` (`self.LapMarker`)))
  (if _returnvalue
    (`MeshComponent.SetScalarParameterValueOnMaterials` (`self.CheckpointViz1`) "checkpointColor" 1.0)
    (`MeshComponent.SetScalarParameterValueOnMaterials` (`self.CheckpointViz2`) "checkpointColor" 1.0)
    ;;[0 0 0] Reset Lap Marker after delay...
    (`KismetSystemLibrary.Delay` 5.0)
    (`MeshComponent.SetScalarParameterValueOnMaterials` (`self.CheckpointViz1`) "checkpointColor" 0.0)
    (`MeshComponent.SetScalarParameterValueOnMaterials` (`self.CheckpointViz2`) "checkpointColor" 0.0)))

(event `self.LapMarker.OnFinish`
  ;[1 1 1] Sparklers on race finished...
  (`ActorComponent.SetActive` (`self.P_Sparks_Left`) true false)
  (`ActorComponent.SetActive` (`self.P_Sparks_Right`) true false)
  (`KismetSystemLibrary.PrintString` "Race Finished!"))

(fn `UserConstructionScript`)