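; Race checkpoint Blueprint that shows whether the sports car has passed it.
; When a BP_SportsCar_Pawn overlaps the CheckpointState component, it calls HitCheckpoint and, if that succeeds, sets the checkpointColor material parameter on two visualizer components.
; CheckpointState's OnResetCheckpoint event, noted as firing on lap completion, switches both visualizers back to their default color.
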(event `self.CheckpointState.OnComponentBeginOverlap`
  (params (OverlappedComponent :type "PrimitiveComponent Object Reference") (OtherActor :type "Actor Object Reference") (OtherComp :type "PrimitiveComponent Object Reference") (OtherBodyIndex :type Integer) (bFromSweep :type Boolean) (SweepResult :type "HitResult Structure (by ref)"))
  ;[1 1 1] On Checkpoint Hit...
  (cast `/Game/VehicleTemplate/Blueprints/SportsCar/BP_SportsCar_Pawn` OtherActor)
  (bind _returnvalue (`CheckpointStateComponent.HitCheckpoint` (`self.CheckpointState`)))
  (if _returnvalue
    (`MeshComponent.SetScalarParameterValueOnMaterials` (`self.CheckpointViz1`) "checkpointColor" 1.0)
    (`MeshComponent.SetScalarParameterValueOnMaterials` (`self.CheckpointViz2`) "checkpointColor" 1.0)))

(event `self.CheckpointState.OnResetCheckpoint`
  ;[1 1 1] On lap complete, reset checkpoitns...
  (`MeshComponent.SetScalarParameterValueOnMaterials` (`self.CheckpointViz1`) "checkpointColor" 0.0)
  (`MeshComponent.SetScalarParameterValueOnMaterials` (`self.CheckpointViz2`) "checkpointColor" 0.0))

(fn `UserConstructionScript`)